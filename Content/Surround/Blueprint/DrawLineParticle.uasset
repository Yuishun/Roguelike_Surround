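; DrawLineParticle is an actor that drives a Niagara effect from a moving particle position, apparently to draw a line.
; While its Active flag is set, Tick passes MParticlePosition to the Niagara User.NewPosition parameter.
; Two DoOnce gates that reset each other activate or deactivate the system only when that flag changes.
; Unwired pause and reset nodes remain unused.
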(event `self.ReceiveBeginPlay`)

(event `self.ReceiveTick`
  (params (DeltaSeconds :type "Float (single-precision)"))
  (if (`DrawLineParticleComponent.bActive` (`self.DrawLineParticle`))
    (`NiagaraComponent.SetNiagaraVariableVec3` (`self.Niagara`) "User.NewPosition" (`DrawLineParticleComponent.m_ParticlePosition` (`self.DrawLineParticle`)))
    (`/Engine/EditorBlueprintResources/StandardMacros.DoOnce` false :!label _label
      (:`Completed`
        (`ActorComponent.Activate` (`self.Niagara`) false)
        (goto _label_2 :!via `Reset`)))
    (else
      (`/Engine/EditorBlueprintResources/StandardMacros.DoOnce` false :!label _label_2
        (:`Completed`
          (`ActorComponent.Deactivate` (`self.Niagara`))
          (goto _label :!via `Reset`))))))

(fn `UserConstructionScript`)