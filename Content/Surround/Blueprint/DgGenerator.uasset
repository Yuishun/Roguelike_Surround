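; DgGenerator is a dungeon generator Blueprint, currently mostly stubbed, that assigns sprites to map tile actors.
; Only SetSpriteWall works: it casts to Wall and picks one of three castle sprites from (X + Y) modulo 3.
; GenerateMap and SpawnMap calls are disconnected, as is the Floor and Road sprite logic.
; GetSpriteFloor and GetSpriteRoad are empty, and BeginPlay does nothing.
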(event `self.ReceiveBeginPlay`)

(event `self.SetSprite_Floor`
  (params (wallActor :type "Actor Object Reference") (walldir :type "DungeonRect Structure")))

(event `self.SetSprite_Road`
  (params (wallActor :type "Actor Object Reference") (walldir :type "DungeonRect Structure")))

(event `self.SetSprite_Wall`
  (params (x :type Integer) (y :type Integer) (wallActor :type "Actor Object Reference"))
  (bind _aswall (cast `/Game/Surround/Blueprint/Wall` wallActor))
  (`PaperSpriteComponent.SetSprite` (`/Game/Surround/Blueprint/Wall.WallSprite` _aswall) (select `int` (mod (+ x y) 3) :`0` "/Game/Surround/Sprite/Map/chip_castle_Sprite_102.chip_castle_Sprite_102" :`1` "/Game/Surround/Sprite/Map/chip_castle_Sprite_104.chip_castle_Sprite_104" :`2` "/Game/Surround/Sprite/Map/chip_castle_Sprite_103.chip_castle_Sprite_103" :!type "PaperSprite Object Reference")))

(fn `GetSprite_Floor`
  (params (WallDir :type "DungeonRect Structure"))
  (returns (Sprite :type "PaperSprite Object Reference"))
  (return null))

(fn `GetSprite_Road`
  (params (WallDir :type "DungeonRect Structure"))
  (returns (Sprite :type "PaperSprite Object Reference"))
  (return null))

(fn `UserConstructionScript`)